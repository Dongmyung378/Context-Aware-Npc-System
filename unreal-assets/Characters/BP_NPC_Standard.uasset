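; Standard NPC character with a daily schedule, trust level, dialogue, trading, random quests and follow behaviour.
; BeginPlay loads data-table stats; Tick compares game time to the schedule, sending the NPC home to hide after hours and ending any following.
; Interact branches on input to open dialogue or shop widgets, resolve item or gold quests, or toggle trust-gated following.
; Blackboard keys pass home, interacting and following states to the AI.
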(event `self.Sphere.OnComponentBeginOverlap`
  (params (OverlappedComponent :type "PrimitiveComponent Object Reference") (OtherActor :type "Actor Object Reference") (OtherComp :type "PrimitiveComponent Object Reference") (OtherBodyIndex :type Integer) (bFromSweep :type Boolean) (SweepResult :type "HitResult Structure (by ref)"))
  (bind _asbp_third_person_character (cast `/Game/ThirdPerson/Blueprints/BP_ThirdPersonCharacter` OtherActor))
  (if (not (`/Game/ThirdPerson/Blueprints/BP_ThirdPersonCharacter.PlayerIsInteracting` _asbp_third_person_character))
    (`SceneComponent.SetVisibility` (`self.InteractionWidget`) true false)))

(event `self.ReceiveTick`
  (params (DeltaSeconds :type "Float (single-precision)"))
  (bind _dialogue_widget_ref (`self.Dialogue_Widget_Ref`))
  (bind _lines (break `/Game/AI/ST_DialogueLines` (`BlueprintMapLibrary.Map_Find` (`self.My_Dialogue_Map`) "NewEnumerator7")))
  (bind (_returnvalue_roll _returnvalue_pitch _returnvalue_yaw) (`KismetMathLibrary.BreakRotator` (`KismetMathLibrary.FindLookAtRotation` (`self.K2_GetActorLocation`) (`self.K2_GetActorLocation` (`GameplayStatics.GetPlayerCharacter` 0)))))
  (bind _output (`|GetArrayItem` _lines (`KismetMathLibrary.RandomIntegerInRange` 0 (`KismetArrayLibrary.Array_LastIndex` _lines))))
  (`|ExecutionSequence`
    (:`then_0`
      (bind _asbp_game_mode (cast `/Game/AI/BP_GameMode` (`GameplayStatics.GetGameMode`)))
      (bind _currenttime (`/Game/AI/BP_GameMode.CurrentTime` _asbp_game_mode))
      (bind (_npc_name _personality_type _widget_color _start_time _end_time _home_location _trust_level _required_trust_follow) (break `/Game/AI/ST_NPC_Data` (stale `self.ReceiveBeginPlay` _output_get)))
      (if (and (>= _currenttime _start_time) (< _currenttime _end_time))
        (`BlackboardComponent.SetValueAsBool` (`AIBlueprintHelperLibrary.GetBlackboard` (`AIBlueprintHelperLibrary.GetAIController` self)) (`self.IsAtHome_Key`) false)
        (`self.SetActorHiddenInGame` false)
        (`self.SetActorEnableCollision` true)
        (else
          (`BlackboardComponent.SetValueAsBool` (`AIBlueprintHelperLibrary.GetBlackboard` (`AIBlueprintHelperLibrary.GetAIController` self)) (`self.IsAtHome_Key`) true)
          (`|AIMoveTo` self _home_location null 10.0
            (:`OnSuccess`
              (`self.SetActorHiddenInGame` true)
              (`self.SetActorEnableCollision` false))))))
    (:`then_1`
      (bind _asbp_game_mode_2 (cast `/Game/AI/BP_GameMode` (`GameplayStatics.GetGameMode`)))
      (bind _currenttime_2 (`/Game/AI/BP_GameMode.CurrentTime` _asbp_game_mode_2))
      (if (and (>= _currenttime_2 _start_time) (< _currenttime_2 _end_time))
        (if (`self.IsInteracting`)
          (`self.K2_SetActorRotation` (`KismetMathLibrary.RInterpTo` (`self.K2_GetActorRotation`) (`KismetMathLibrary.MakeRotator` 0.0 0.0 _returnvalue_yaw) DeltaSeconds 5.0)))))
    (:`then_2`
      (bind _asbp_game_mode_3 (cast `/Game/AI/BP_GameMode` (`GameplayStatics.GetGameMode`)))
      (bind _currenttime_3 (`/Game/AI/BP_GameMode.CurrentTime` _asbp_game_mode_3))
      (if (and (>= _currenttime_3 _start_time) (< _currenttime_3 _end_time))
        _
        (elif (`self.IsFollowing`)
          (bind _asbp_third_person_character (cast `/Game/ThirdPerson/Blueprints/BP_ThirdPersonCharacter` (`GameplayStatics.GetPlayerCharacter` 0)))
          (if (`/Game/ThirdPerson/Blueprints/BP_ThirdPersonCharacter.PlayerIsInteracting` _asbp_third_person_character)
            (set `self.IsFollowing` false)
            (`/Engine/EditorBlueprintResources/StandardMacros.IsValid` _dialogue_widget_ref
              (:`Is Valid`
                (`Widget.SetVisibility` (`/Game/AI/WBP_Dialogue.Txt_Key_R` _dialogue_widget_ref) "Hidden")
                (`Widget.SetVisibility` (`/Game/AI/WBP_Dialogue.Txt_Key_T` _dialogue_widget_ref) "Hidden")
                (`Widget.SetVisibility` (`/Game/AI/WBP_Dialogue.Txt_Key_F` _dialogue_widget_ref) "Hidden")
                (`TextBlock.SetText` (`/Game/AI/WBP_Dialogue.Text_Content` _dialogue_widget_ref) _output)
                (set `self.InteractionEnd` true)
                (`KismetSystemLibrary.Delay` 5.0)
                (`/Engine/EditorBlueprintResources/StandardMacros.IsValid` (`self.Dialogue_Widget_Ref`)
                  (:`Is Valid`
                    (bind _asbp_third_person_character_2 (cast `/Game/ThirdPerson/Blueprints/BP_ThirdPersonCharacter` (`GameplayStatics.GetPlayerCharacter` 0)))
                    (set `/Game/ThirdPerson/Blueprints/BP_ThirdPersonCharacter.PlayerIsInteracting` false _asbp_third_person_character_2)
                    (`Widget.RemoveFromParent` (`self.Dialogue_Widget_Ref`))
                    (set `self.Dialogue_Widget_Ref` null))))
              (:`Is Not Valid`
                _))
            (`BlackboardComponent.SetValueAsBool` (`AIBlueprintHelperLibrary.GetBlackboard` (`AIBlueprintHelperLibrary.GetAIController` self)) "IsFollowing" false)
            (set `self.InteractionEnd` false)
            (set `self.IsInteracting` false)
            (else
              (bind _returnvalue (`|CreateWidget` "/Game/AI/WBP_Dialogue.WBP_Dialogue_C"))
              (bind _asbp_third_person_character_3 (cast `/Game/ThirdPerson/Blueprints/BP_ThirdPersonCharacter` (`GameplayStatics.GetPlayerCharacter` 0)))
              (set `/Game/ThirdPerson/Blueprints/BP_ThirdPersonCharacter.PlayerIsInteracting` true _asbp_third_person_character_3)
              (set `self.IsInteracting` true)
              (set `self.InteractionEnd` true)
              (bind _output_get (set `self.Dialogue_Widget_Ref` _returnvalue))
              (`Widget.SetVisibility` (`/Game/AI/WBP_Dialogue.Txt_Key_R` _output_get) "Hidden")
              (`Widget.SetVisibility` (`/Game/AI/WBP_Dialogue.Txt_Key_T` _output_get) "Hidden")
              (`Widget.SetVisibility` (`/Game/AI/WBP_Dialogue.Txt_Key_F` _output_get) "Hidden")
              (`TextBlock.SetText` (`/Game/AI/WBP_Dialogue.Text_Name` _output_get) _npc_name)
              (`TextBlock.SetText` (`/Game/AI/WBP_Dialogue.Txt_TrustLevel` _output_get) (`|FormatText` "Trust: {Trust}" (`self.Trust_Level`)))
              (`TextBlock.SetText` (`/Game/AI/WBP_Dialogue.Text_Content` _output_get) _output)
              (`UserWidget.AddToViewport` _output_get 0)
              (`WidgetBlueprintLibrary.SetInputMode_GameAndUIEx` (`GameplayStatics.GetPlayerController` 0) _output_get)
              (`BlackboardComponent.SetValueAsBool` (`AIBlueprintHelperLibrary.GetBlackboard` (`AIBlueprintHelperLibrary.GetAIController` self)) "IsFollowing" false)
              (set `self.IsFollowing` false)
              (`KismetSystemLibrary.Delay` 5.0)
              (`/Engine/EditorBlueprintResources/StandardMacros.IsValid` (`self.Dialogue_Widget_Ref`)
                (:`Is Valid`
                  (bind _asbp_third_person_character_4 (cast `/Game/ThirdPerson/Blueprints/BP_ThirdPersonCharacter` (`GameplayStatics.GetPlayerCharacter` 0)))
                  (set `/Game/ThirdPerson/Blueprints/BP_ThirdPersonCharacter.PlayerIsInteracting` false _asbp_third_person_character_4)
                  (`Widget.RemoveFromParent` (`self.Dialogue_Widget_Ref`))
                  (set `self.Dialogue_Widget_Ref` null)
                  (set `self.InteractionEnd` false)
                  (set `self.IsInteracting` false))))))))))

(event `self.Sphere.OnComponentEndOverlap`
  (params (OverlappedComponent :type "PrimitiveComponent Object Reference") (OtherActor :type "Actor Object Reference") (OtherComp :type "PrimitiveComponent Object Reference") (OtherBodyIndex :type Integer))
  (bind _returnvalue (`GameplayStatics.GetPlayerController` 0))
  (bind _shop_widget_ref (`self.Shop_Widget_Ref`))
  (cast `/Game/ThirdPerson/Blueprints/BP_ThirdPersonCharacter` OtherActor)
  (`SceneComponent.SetVisibility` (`self.InteractionWidget`) false false)
  (if (`self.IsInteracting`)
    (`/Engine/EditorBlueprintResources/StandardMacros.IsValid` (`self.Dialogue_Widget_Ref`)
      (:`Is Valid`
        (`Widget.RemoveFromParent` (`self.Dialogue_Widget_Ref`)))
      (:`Is Not Valid`
        _))
    (`/Engine/EditorBlueprintResources/StandardMacros.IsValid` _shop_widget_ref
      (:`Is Valid`
        (`Widget.RemoveFromParent` _shop_widget_ref))
      (:`Is Not Valid`
        _))
    (bind _asbp_third_person_character (cast `/Game/ThirdPerson/Blueprints/BP_ThirdPersonCharacter` (`GameplayStatics.GetPlayerCharacter` 0)))
    (set `/Game/ThirdPerson/Blueprints/BP_ThirdPersonCharacter.PlayerIsInteracting` false _asbp_third_person_character)
    (set `self.IsInteracting` false)
    (set `self.InteractionEnd` false)
    (`BlackboardComponent.SetValueAsBool` (`AIBlueprintHelperLibrary.GetBlackboard` (`AIBlueprintHelperLibrary.GetAIController` self)) "IsInteracting" false)
    (`WidgetBlueprintLibrary.SetInputMode_GameOnly` _returnvalue)
    (set `PlayerController.bShowMouseCursor` false _returnvalue)
    (set `self.Dialogue_Widget_Ref` null)
    (set `self.Shop_Widget_Ref` null)))

(event `self.ReceiveActorBeginOverlap`
  (params (OtherActor :type "Actor Object Reference")))

(event `self.ReceiveBeginPlay`
  (bind _returnvalue (`|GetDataTableRow` "/Game/AI/DT_NPC_Data.DT_NPC_Data" (`self.NPC_Row_Name`))
    (:`then`
      (bind _output_get (set `self.My_NPC_Data` _returnvalue))
      (set `self.Trust_Level` (`.Trust_Level_44_7A4EA0BF4C8DB7AA23A30DABD1F69FAA` (break `/Game/AI/ST_NPC_Data` _output_get))))))

(event `/Game/AI/BPI_Interaction.Interact`
  (params (InteractionKey :type Name))
  (bind _returnvalue (`GameplayStatics.GetPlayerController` 0))
  (bind _returnvalue_2 (`GameplayStatics.GetPlayerController` 0))
  (bind _dialogue_widget_ref (`self.Dialogue_Widget_Ref`))
  (bind _dialogue_widget_ref_2 (`self.Dialogue_Widget_Ref`))
  (bind _trust_level (`self.Trust_Level`))
  (bind _shop_widget_ref (`self.Shop_Widget_Ref`))
  (bind _my_dialogue_map (`self.My_Dialogue_Map`))
  (bind _dialogue_widget_ref_3 (`self.Dialogue_Widget_Ref`))
  (bind _my_dialogue_map_2 (`self.My_Dialogue_Map`))
  (bind _dialogue_widget_ref_4 (`self.Dialogue_Widget_Ref`))
  (bind _my_dialogue_map_3 (`self.My_Dialogue_Map`))
  (bind _target_index (`self.Target_Index`))
  (bind (_quest_name _quest_type _target_item _target_amount _reward_gold _reward_trust) (break `/Game/AI/ST_QuestData` (`self.ActiveQuest`)))
  (bind _text_content (`/Game/AI/WBP_Dialogue.Text_Content` _dialogue_widget_ref))
  (bind _text_content_2 (`/Game/AI/WBP_Dialogue.Text_Content` _dialogue_widget_ref_3))
  (bind _txt_key_r (`/Game/AI/WBP_Dialogue.Txt_Key_R` _dialogue_widget_ref_3))
  (bind _text_content_3 (`/Game/AI/WBP_Dialogue.Text_Content` _dialogue_widget_ref_4))
  (bind _txt_key_r_2 (`/Game/AI/WBP_Dialogue.Txt_Key_R` _dialogue_widget_ref_4))
  (bind _txt_key_r_3 (`/Game/AI/WBP_Dialogue.Txt_Key_R` _dialogue_widget_ref))
  (bind _lines (break `/Game/AI/ST_DialogueLines` (`BlueprintMapLibrary.Map_Find` (`self.My_Dialogue_Map`) "NewEnumerator14")))
  (bind _lines_2 (break `/Game/AI/ST_DialogueLines` (`BlueprintMapLibrary.Map_Find` _my_dialogue_map_3 "NewEnumerator20")))
  (bind _lines_3 (break `/Game/AI/ST_DialogueLines` (`BlueprintMapLibrary.Map_Find` _my_dialogue_map_2 "NewEnumerator16")))
  (bind _lines_4 (break `/Game/AI/ST_DialogueLines` (`BlueprintMapLibrary.Map_Find` _my_dialogue_map "NewEnumerator4")))
  (bind _lines_5 (break `/Game/AI/ST_DialogueLines` (`BlueprintMapLibrary.Map_Find` _my_dialogue_map_3 "NewEnumerator19")))
  (bind _lines_6 (break `/Game/AI/ST_DialogueLines` (`BlueprintMapLibrary.Map_Find` _my_dialogue_map_2 "NewEnumerator15")))
  (bind _lines_7 (break `/Game/AI/ST_DialogueLines` (`BlueprintMapLibrary.Map_Find` (`self.My_Dialogue_Map`) "NewEnumerator7")))
  (bind _lines_8 (break `/Game/AI/ST_DialogueLines` (`BlueprintMapLibrary.Map_Find` _my_dialogue_map "NewEnumerator11")))
  (bind _lines_9 (break `/Game/AI/ST_DialogueLines` (`BlueprintMapLibrary.Map_Find` _my_dialogue_map_2 "NewEnumerator17")))
  (bind _lines_10 (break `/Game/AI/ST_DialogueLines` (`BlueprintMapLibrary.Map_Find` _my_dialogue_map_3 "NewEnumerator18")))
  (bind _returnvalue_3 (- (`self.Target_Quantity`) _target_amount))
  (bind _output (`|GetArrayItem` _lines (`KismetMathLibrary.RandomIntegerInRange` 0 (`KismetArrayLibrary.Array_LastIndex` _lines))))
  (switch `name` InteractionKey
    (:`Interact`
      (bind _asbp_game_mode (cast `/Game/AI/BP_GameMode` (`GameplayStatics.GetGameMode`)))
      (bind _currenttime (`/Game/AI/BP_GameMode.CurrentTime` _asbp_game_mode))
      (bind (_npc_name _personality_type _widget_color _start_time _end_time _home_location _trust_level_2 _required_trust_follow) (break `/Game/AI/ST_NPC_Data` (stale `self.ReceiveBeginPlay` _output_get)))
      (if (and (>= _currenttime _start_time) (< _currenttime _end_time))
        (if (`self.IsInteracting`)
          (bind _asbp_third_person_character (cast `/Game/ThirdPerson/Blueprints/BP_ThirdPersonCharacter` (`GameplayStatics.GetPlayerCharacter` 0) :!label _label))
          (if (`/Game/ThirdPerson/Blueprints/BP_ThirdPersonCharacter.PlayerIsInteracting` _asbp_third_person_character)
            (set `/Game/ThirdPerson/Blueprints/BP_ThirdPersonCharacter.PlayerIsInteracting` false _asbp_third_person_character)
            (`/Engine/EditorBlueprintResources/StandardMacros.IsValid` (`self.Dialogue_Widget_Ref`)
              (:`Is Valid`
                (set `self.IsInteracting` false)
                (`BlackboardComponent.SetValueAsBool` (`AIBlueprintHelperLibrary.GetBlackboard` (`AIBlueprintHelperLibrary.GetAIController` self)) "IsInteracting" false)
                (`Widget.RemoveFromParent` (`self.Dialogue_Widget_Ref`))
                (`/Engine/EditorBlueprintResources/StandardMacros.IsValid` _shop_widget_ref
                  (:`Is Valid`
                    (`Widget.RemoveFromParent` _shop_widget_ref))
                  (:`Is Not Valid`
                    _))
                (`WidgetBlueprintLibrary.SetInputMode_GameOnly` _returnvalue_2)
                (set `PlayerController.bShowMouseCursor` false _returnvalue_2)
                (set `self.Dialogue_Widget_Ref` null)
                (set `self.InteractionEnd` false)
                (set `self.Shop_Widget_Ref` null))))
          (else
            (bind _asbp_third_person_character_2 (cast `/Game/ThirdPerson/Blueprints/BP_ThirdPersonCharacter` (`GameplayStatics.GetPlayerCharacter` 0)))
            (if (not (`/Game/ThirdPerson/Blueprints/BP_ThirdPersonCharacter.PlayerIsInteracting` _asbp_third_person_character_2))
              (set `/Game/ThirdPerson/Blueprints/BP_ThirdPersonCharacter.PlayerIsInteracting` true _asbp_third_person_character_2)
              (bind _returnvalue_4 (`|CreateWidget` "/Game/AI/WBP_Dialogue.WBP_Dialogue_C"))
              (set `self.IsInteracting` true)
              (`BlackboardComponent.SetValueAsBool` (`AIBlueprintHelperLibrary.GetBlackboard` (`AIBlueprintHelperLibrary.GetAIController` self)) "IsInteracting" true)
              (bind _output_get (set `self.Dialogue_Widget_Ref` _returnvalue_4))
              (`Widget.SetVisibility` (`/Game/AI/WBP_Dialogue.Txt_Key_E` _output_get) "Visible")
              (`Widget.SetVisibility` (`/Game/AI/WBP_Dialogue.Txt_Key_R` _output_get) "Visible")
              (`Widget.SetVisibility` (`/Game/AI/WBP_Dialogue.Txt_Key_T` _output_get) "Visible")
              (`Widget.SetVisibility` (`/Game/AI/WBP_Dialogue.Txt_Key_F` _output_get) "Visible")
              (`TextBlock.SetText` (`/Game/AI/WBP_Dialogue.Text_Name` _output_get) _npc_name)
              (`TextBlock.SetText` (`/Game/AI/WBP_Dialogue.Txt_TrustLevel` _output_get) (`|FormatText` "Trust: {Trust}" _trust_level))
              (if (>= _trust_level _required_trust_follow)
                (bind _text_content_4 (`/Game/AI/WBP_Dialogue.Text_Content` _output_get))
                (`TextBlock.SetText` _text_content_4 (`|GetArrayItem` _lines_8 (`KismetMathLibrary.RandomIntegerInRange` 0 (`KismetArrayLibrary.Array_LastIndex` _lines_8))))
                (else
                  (`TextBlock.SetText` _text_content_4 (`|GetArrayItem` _lines_4 (`KismetMathLibrary.RandomIntegerInRange` 0 (`KismetArrayLibrary.Array_LastIndex` _lines_4))))))
              (`UserWidget.AddToViewport` _output_get 0)
              (`WidgetBlueprintLibrary.SetInputMode_GameAndUIEx` (`GameplayStatics.GetPlayerController` 0) _output_get))))
        (else
          (`/Engine/EditorBlueprintResources/StandardMacros.IsValid` (`self.Dialogue_Widget_Ref`)
            (:`Is Valid`
              (goto _label))
            (:`Is Not Valid`
              (bind _asbp_third_person_character_3 (cast `/Game/ThirdPerson/Blueprints/BP_ThirdPersonCharacter` (`GameplayStatics.GetPlayerCharacter` 0)))
              (if (not (`/Game/ThirdPerson/Blueprints/BP_ThirdPersonCharacter.PlayerIsInteracting` _asbp_third_person_character_3))
                (set `/Game/ThirdPerson/Blueprints/BP_ThirdPersonCharacter.PlayerIsInteracting` true _asbp_third_person_character_3)
                (bind _returnvalue_5 (`|CreateWidget` "/Game/AI/WBP_Dialogue.WBP_Dialogue_C"))
                (bind _output_get_2 (set `self.Dialogue_Widget_Ref` _returnvalue_5))
                (`Widget.SetVisibility` (`/Game/AI/WBP_Dialogue.Txt_Key_R` _output_get_2) "Hidden")
                (`Widget.SetVisibility` (`/Game/AI/WBP_Dialogue.Txt_Key_T` _output_get_2) "Hidden")
                (`Widget.SetVisibility` (`/Game/AI/WBP_Dialogue.Txt_Key_F` _output_get_2) "Hidden")
                (`TextBlock.SetText` (`/Game/AI/WBP_Dialogue.Text_Name` _output_get_2) _npc_name)
                (`TextBlock.SetText` (`/Game/AI/WBP_Dialogue.Txt_TrustLevel` _output_get_2) (`|FormatText` "Trust: {Trust}" (`self.Trust_Level`)))
                (`TextBlock.SetText` (`/Game/AI/WBP_Dialogue.Text_Content` _output_get_2) (`|GetArrayItem` _lines_7 (`KismetMathLibrary.RandomIntegerInRange` 0 (`KismetArrayLibrary.Array_LastIndex` _lines_7))))
                (`UserWidget.AddToViewport` _output_get_2 0)
                (`WidgetBlueprintLibrary.SetInputMode_GameAndUIEx` (`GameplayStatics.GetPlayerController` 0) _output_get_2)
                (`KismetSystemLibrary.Delay` 5.0)
                (`/Engine/EditorBlueprintResources/StandardMacros.IsValid` (`self.Dialogue_Widget_Ref`)
                  (:`Is Valid`
                    (bind _asbp_third_person_character_4 (cast `/Game/ThirdPerson/Blueprints/BP_ThirdPersonCharacter` (`GameplayStatics.GetPlayerCharacter` 0)))
                    (set `/Game/ThirdPerson/Blueprints/BP_ThirdPersonCharacter.PlayerIsInteracting` false _asbp_third_person_character_4)
                    (`Widget.RemoveFromParent` (`self.Dialogue_Widget_Ref`))
                    (set `self.Dialogue_Widget_Ref` null)))))))))
    (:`Talk`
      (if (`self.InteractionEnd`)
        _
        (elif (`self.IsInteracting`)
          (if (`self.QuestStatus`)
            (bind _asbp_third_person_character_5 (cast `/Game/ThirdPerson/Blueprints/BP_ThirdPersonCharacter` (`GameplayStatics.GetPlayerCharacter` 0)))
            (switch `/Game/AI/E_QuestType` _quest_type
              (:`NewEnumerator0`
                (set `self.CheckQuestCondition` false)
                (bind _inventory (`/Game/ThirdPerson/Blueprints/BP_ThirdPersonCharacter.Inventory` _asbp_third_person_character_5))
                (for (_array_element _array_index) _inventory
                  (bind (_item_name _item_mesh _material _item_type _is_rare _item_price _trust_point _count) (break `/Game/AI/ST_Item_Data` _array_element))
                  (if (`KismetTextLibrary.EqualEqual_TextText` _item_name (`KismetTextLibrary.Conv_NameToText` _target_item))
                    (if (>= _count _target_amount)
                      (set `self.CheckQuestCondition` true)
                      (set `self.Target_Index` _array_index)
                      (set `self.Target_Quantity` _count)
                      (break))))
                (if (`self.CheckQuestCondition`)
                  (if (== _returnvalue_3 0)
                    (`KismetArrayLibrary.Array_Remove` _inventory _target_index)
                    (else
                      (bind _structout (setmembers `/Game/AI/ST_Item_Data` :`StructRef` (`|GetArrayItem` _inventory _target_index) :`Count` _returnvalue_3))
                      (`KismetArrayLibrary.Array_Set` _inventory _target_index _structout true)))
                  (set `/Game/ThirdPerson/Blueprints/BP_ThirdPersonCharacter.Money` (+ (`/Game/ThirdPerson/Blueprints/BP_ThirdPersonCharacter.Money` _asbp_third_person_character_5) _reward_gold) _asbp_third_person_character_5)
                  (set `self.Trust_Level` (+ (`self.Trust_Level`) _reward_trust))
                  (set `self.QuestStatus` false)
                  (`Widget.SetVisibility` _txt_key_r_2 "Hidden")
                  (`Widget.SetVisibility` (`/Game/AI/WBP_Dialogue.Txt_Key_T` _dialogue_widget_ref_4) "Hidden")
                  (`Widget.SetVisibility` (`/Game/AI/WBP_Dialogue.Txt_Key_F` _dialogue_widget_ref_4) "Hidden")
                  (`TextBlock.SetText` _text_content_3 _output)
                  (set `self.InteractionEnd` true)
                  (else
                    (`Widget.SetVisibility` _txt_key_r_2 "Hidden")
                    (`Widget.SetVisibility` (`/Game/AI/WBP_Dialogue.Txt_Key_T` _dialogue_widget_ref_4) "Hidden")
                    (`Widget.SetVisibility` (`/Game/AI/WBP_Dialogue.Txt_Key_F` _dialogue_widget_ref_4) "Hidden")
                    (`TextBlock.SetText` _text_content_3 (`|FormatText` "The quest isn't finished yet. I still need {Count} {ItemName}(s) from you." _target_amount _target_item))
                    (set `self.InteractionEnd` true))))
              (:`NewEnumerator1`
                (bind _money (`/Game/ThirdPerson/Blueprints/BP_ThirdPersonCharacter.Money` _asbp_third_person_character_5))
                (if (>= _money _target_amount)
                  (set `/Game/ThirdPerson/Blueprints/BP_ThirdPersonCharacter.Money` (- _money _target_amount) _asbp_third_person_character_5)
                  (set `self.Trust_Level` (+ (`self.Trust_Level`) _reward_trust))
                  (set `self.QuestStatus` false)
                  (`Widget.SetVisibility` _txt_key_r_2 "Hidden")
                  (`Widget.SetVisibility` (`/Game/AI/WBP_Dialogue.Txt_Key_T` _dialogue_widget_ref_4) "Hidden")
                  (`Widget.SetVisibility` (`/Game/AI/WBP_Dialogue.Txt_Key_F` _dialogue_widget_ref_4) "Hidden")
                  (`TextBlock.SetText` _text_content_3 _output)
                  (set `self.InteractionEnd` true)
                  (else
                    (`Widget.SetVisibility` _txt_key_r_2 "Hidden")
                    (`Widget.SetVisibility` (`/Game/AI/WBP_Dialogue.Txt_Key_T` _dialogue_widget_ref_4) "Hidden")
                    (`Widget.SetVisibility` (`/Game/AI/WBP_Dialogue.Txt_Key_F` _dialogue_widget_ref_4) "Hidden")
                    (`TextBlock.SetText` _text_content_3 (`|FormatText` "I still need {Amount} money to finish this." _target_amount))
                    (set `self.InteractionEnd` true)))))
            (elif (<= (`KismetMathLibrary.RandomFloatInRange` 0.0 1.0) 0.1)
              (bind _outrownames (`DataTableFunctionLibrary.GetDataTableRowNames` "/Game/AI/DT_QuestList.DT_QuestList"))
              (bind _returnvalue_6 (`|GetDataTableRow` "/Game/AI/DT_QuestList.DT_QuestList" (`KismetArrayLibrary.Array_Random` _outrownames))
                (:`then`
                  (bind _output_get_3 (set `self.ActiveQuest` _returnvalue_6))
                  (set `self.QuestStatus` true)
                  (`Widget.SetVisibility` _txt_key_r_3 "Hidden")
                  (`Widget.SetVisibility` (`/Game/AI/WBP_Dialogue.Txt_Key_T` _dialogue_widget_ref) "Hidden")
                  (`Widget.SetVisibility` (`/Game/AI/WBP_Dialogue.Txt_Key_F` _dialogue_widget_ref) "Hidden")
                  (`TextBlock.SetText` _text_content (`.Quest_Description_17_83613C6C45E0D69FF774E781DFCD3B83` (break `/Game/AI/ST_QuestData` _output_get_3)))
                  (set `self.InteractionEnd` true)))
              (else
                (bind _asbp_third_person_character_6 (cast `/Game/ThirdPerson/Blueprints/BP_ThirdPersonCharacter` (`GameplayStatics.GetPlayerCharacter` 0)))
                (if (<= (`/Game/ThirdPerson/Blueprints/BP_ThirdPersonCharacter.Current_Stamina` _asbp_third_person_character_6) 30.0)
                  (`Widget.SetVisibility` _txt_key_r_3 "Hidden")
                  (`Widget.SetVisibility` (`/Game/AI/WBP_Dialogue.Txt_Key_T` _dialogue_widget_ref) "Hidden")
                  (`Widget.SetVisibility` (`/Game/AI/WBP_Dialogue.Txt_Key_F` _dialogue_widget_ref) "Hidden")
                  (`TextBlock.SetText` _text_content (`|GetArrayItem` _lines_2 (`KismetMathLibrary.RandomIntegerInRange` 0 (`KismetArrayLibrary.Array_LastIndex` _lines_2))))
                  (set `self.InteractionEnd` true)
                  (elif (== (`/Game/ThirdPerson/Blueprints/BP_ThirdPersonCharacter.Money` _asbp_third_person_character_6) 0)
                    (`Widget.SetVisibility` _txt_key_r_3 "Hidden")
                    (`Widget.SetVisibility` (`/Game/AI/WBP_Dialogue.Txt_Key_T` _dialogue_widget_ref) "Hidden")
                    (`Widget.SetVisibility` (`/Game/AI/WBP_Dialogue.Txt_Key_F` _dialogue_widget_ref) "Hidden")
                    (`TextBlock.SetText` _text_content (`|GetArrayItem` _lines_5 (`KismetMathLibrary.RandomIntegerInRange` 0 (`KismetArrayLibrary.Array_LastIndex` _lines_5))))
                    (set `self.InteractionEnd` true)
                    (else
                      (`Widget.SetVisibility` _txt_key_r_3 "Hidden")
                      (`Widget.SetVisibility` (`/Game/AI/WBP_Dialogue.Txt_Key_T` _dialogue_widget_ref) "Hidden")
                      (`Widget.SetVisibility` (`/Game/AI/WBP_Dialogue.Txt_Key_F` _dialogue_widget_ref) "Hidden")
                      (`TextBlock.SetText` _text_content (`|GetArrayItem` _lines_10 (`KismetMathLibrary.RandomIntegerInRange` 0 (`KismetArrayLibrary.Array_LastIndex` _lines_10))))
                      (set `self.InteractionEnd` true))))))))))
    (:`Trade`
      (if (`self.InteractionEnd`)
        _
        (elif (`self.IsInteracting`)
          (`/Engine/EditorBlueprintResources/StandardMacros.IsValid` _dialogue_widget_ref_2
            (:`Is Valid`
              (`Widget.RemoveFromParent` _dialogue_widget_ref_2))
            (:`Is Not Valid`
              _))
          (bind _returnvalue_7 (`|CreateWidget` "/Game/AI/WBP_ShopMain.WBP_ShopMain_C" null self))
          (bind _output_get_4 (set `self.Shop_Widget_Ref` _returnvalue_7))
          (bind _npc_saleslist (`/Game/AI/WBP_ShopMain.NPC_SalesList` _output_get_4))
          (`KismetArrayLibrary.Array_Clear` _npc_saleslist)
          (for _array_element_2 (`self.ItemsToSell`)
            (bind _returnvalue_8 (`|GetDataTableRow` "/Game/AI/DT_Item_Data.DT_Item_Data" _array_element_2)
              (:`then`
                (`KismetArrayLibrary.Array_Add` _npc_saleslist _returnvalue_8))))
          (`/Game/AI/WBP_ShopMain.UpdateShopUI` _output_get_4)
          (`UserWidget.AddToViewport` _output_get_4 0)
          (set `PlayerController.bShowMouseCursor` true _returnvalue)
          (`WidgetBlueprintLibrary.SetInputMode_GameAndUIEx` _returnvalue _output_get_4)
          (set `self.InteractionEnd` true))))
    (:`Follow`
      (if (`self.InteractionEnd`)
        _
        (elif (`self.IsInteracting`)
          (if (`self.IsFollowing`)
            (set `self.IsFollowing` false)
            (`Widget.SetVisibility` _txt_key_r "Hidden")
            (`Widget.SetVisibility` (`/Game/AI/WBP_Dialogue.Txt_Key_T` _dialogue_widget_ref_3) "Hidden")
            (`Widget.SetVisibility` (`/Game/AI/WBP_Dialogue.Txt_Key_F` _dialogue_widget_ref_3) "Hidden")
            (`TextBlock.SetText` _text_content_2 (`|GetArrayItem` _lines_9 (`KismetMathLibrary.RandomIntegerInRange` 0 (`KismetArrayLibrary.Array_LastIndex` _lines_9))))
            (`BlackboardComponent.SetValueAsBool` (`AIBlueprintHelperLibrary.GetBlackboard` (`AIBlueprintHelperLibrary.GetAIController` self)) "IsFollowing" false)
            (set `self.InteractionEnd` true)
            (elif (>= (`self.Trust_Level`) _required_trust_follow)
              (set `self.IsFollowing` true)
              (`Widget.SetVisibility` _txt_key_r "Hidden")
              (`Widget.SetVisibility` (`/Game/AI/WBP_Dialogue.Txt_Key_T` _dialogue_widget_ref_3) "Hidden")
              (`Widget.SetVisibility` (`/Game/AI/WBP_Dialogue.Txt_Key_F` _dialogue_widget_ref_3) "Hidden")
              (`TextBlock.SetText` _text_content_2 (`|GetArrayItem` _lines_6 (`KismetMathLibrary.RandomIntegerInRange` 0 (`KismetArrayLibrary.Array_LastIndex` _lines_6))))
              (`BlackboardComponent.SetValueAsBool` (`AIBlueprintHelperLibrary.GetBlackboard` (`AIBlueprintHelperLibrary.GetAIController` self)) "IsFollowing" true)
              (set `self.InteractionEnd` true)
              (else
                (`Widget.SetVisibility` _txt_key_r "Hidden")
                (`Widget.SetVisibility` (`/Game/AI/WBP_Dialogue.Txt_Key_T` _dialogue_widget_ref_3) "Hidden")
                (`Widget.SetVisibility` (`/Game/AI/WBP_Dialogue.Txt_Key_F` _dialogue_widget_ref_3) "Hidden")
                (`TextBlock.SetText` _text_content_2 (`|GetArrayItem` _lines_3 (`KismetMathLibrary.RandomIntegerInRange` 0 (`KismetArrayLibrary.Array_LastIndex` _lines_3))))
                (set `self.InteractionEnd` true)))))))))

(fn `Update Walk Speed`
  (params (NewSpeed :type "Float (double-precision)"))
  (set `CharacterMovementComponent.MaxWalkSpeed` NewSpeed (`self.CharacterMovement`)))

(fn `UserConstructionScript`)