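; Game mode that adds the clock, stamina, money and dash HUD widget and runs the day-night clock with time-based ambient music.
; Tick advances CurrentTime by a speed multiplier, wrapping every 24 hours.
; Morning, midday and night windows each start their own 2D track through chained DoOnce gates that re-arm the next, fading out the previous track.
; Outside these windows, Tick repeatedly calls FadeOut on the active track.
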(event `self.ReceiveBeginPlay`
  (bind _returnvalue (`|CreateWidget` "/Game/AI/WBP_Clock_Stamina_Money_Dash.WBP_Clock_Stamina_Money_Dash_C"))
  (`UserWidget.AddToViewport` _returnvalue 0))

(event `self.ReceiveTick`
  (params (DeltaSeconds :type "Float (single-precision)"))
  (bind _activebgm (`self.ActiveBGM`))
  (bind _output_get (set `self.CurrentTime` (mod (+ (* DeltaSeconds (`self.TimeSpeed`)) (`self.CurrentTime`)) 1440.0)))
  (bind _returnvalue (/ _output_get 60.0))
  (if (and (>= _returnvalue 6.0) (< _returnvalue 7.0))
    (`/Engine/EditorBlueprintResources/StandardMacros.DoOnce` false :!label _label
      (:`Completed`
        (`/Engine/EditorBlueprintResources/StandardMacros.IsValid` _activebgm
          (:`Is Valid`
            (`AudioComponent.FadeOut` _activebgm 2.0 0.0 "Linear"))
          (:`Is Not Valid`
            _))
        (bind _returnvalue_2 (`GameplayStatics.SpawnSound2D` "/Game/A001_ForestSounds/Audios/ENV/ENV_Day_BirdsChirping2.ENV_Day_BirdsChirping2" 1.0 1.0 0.0 null))
        (set `self.ActiveBGM` _returnvalue_2)
        (goto _label_2 :!via `Reset`)))
    (else
      (bind _returnvalue_3 (/ _output_get 60.0))
      (if (and (>= _returnvalue_3 11.0) (< _returnvalue_3 14.0))
        (`/Engine/EditorBlueprintResources/StandardMacros.DoOnce` false :!label _label_2
          (:`Completed`
            (`/Engine/EditorBlueprintResources/StandardMacros.IsValid` _activebgm
              (:`Is Valid`
                (`AudioComponent.FadeOut` _activebgm 2.0 0.0 "Linear"))
              (:`Is Not Valid`
                _))
            (bind _returnvalue_4 (`GameplayStatics.SpawnSound2D` "/Game/A001_ForestSounds/Audios/ENV/ENV_Day_MossyGroundShift2.ENV_Day_MossyGroundShift2" 1.0 1.0 0.0 null))
            (set `self.ActiveBGM` _returnvalue_4)
            (goto _label_3 :!via `Reset`)))
        (elif (>= (/ _output_get 60.0) 20.0)
          (`/Engine/EditorBlueprintResources/StandardMacros.DoOnce` false :!label _label_3
            (:`Completed`
              (`/Engine/EditorBlueprintResources/StandardMacros.IsValid` _activebgm
                (:`Is Valid`
                  (`AudioComponent.FadeOut` _activebgm 2.0 0.0 "Linear"))
                (:`Is Not Valid`
                  _))
              (bind _returnvalue_5 (`GameplayStatics.SpawnSound2D` "/Game/A001_ForestSounds/Audios/ENV/ENV_Night_MoonlitAmbience1.ENV_Night_MoonlitAmbience1" 1.0 1.0 0.0 null))
              (set `self.ActiveBGM` _returnvalue_5)
              (goto _label :!via `Reset`)))
          (else
            (`/Engine/EditorBlueprintResources/StandardMacros.IsValid` _activebgm
              (:`Is Valid`
                (`AudioComponent.FadeOut` _activebgm 2.0 0.0 "Linear")))))))))

(fn `UserConstructionScript`)