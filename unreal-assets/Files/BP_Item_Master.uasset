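; Master pickup item actor that players collect into their inventory, respawning after a delay.
; On BeginPlay it looks up its item in DT_Item_Data, with a small chance of using the "Rare_" row variant, and applies mesh and material.
; Overlap enables input and a Take prompt; E stacks or adds the item and refreshes the inventory widget.
; The actor then hides without collision, and later reappears with a rerolled rarity.
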(event `DecideItem`
  (bind _staticmesh (`self.StaticMesh`))
  (if (<= (`KismetMathLibrary.RandomFloatInRange` 0.0 1.0) 0.1)
    (set `self.Final_ID` (`KismetStringLibrary.Conv_StringToName` (`KismetStringLibrary.Concat_StrStr` "Rare_" (`KismetStringLibrary.Conv_NameToString` (`self.Item_ID`)))))
    (else
      (bind _output_get (set `self.Final_ID` (`self.Item_ID`)))))
  (bind _returnvalue (`|GetDataTableRow` "/Game/AI/DT_Item_Data.DT_Item_Data" _output_get)
    (:`then`
      (bind _output_get_2 (set `self.MyItemData` _returnvalue))
      (bind (_item_name _item_mesh _material) (break `/Game/AI/ST_Item_Data` _output_get_2))
      (`StaticMeshComponent.SetStaticMesh` _staticmesh _item_mesh)
      (`PrimitiveComponent.SetMaterial` _staticmesh 0 _material))))

(event `self.ReceiveBeginPlay`
  (`self.DecideItem`))

(event `self.ReceiveActorBeginOverlap`
  (params (OtherActor :type "Actor Object Reference"))
  (bind _asbp_third_person_character (cast `/Game/ThirdPerson/Blueprints/BP_ThirdPersonCharacter` OtherActor))
  (if (not (`/Game/ThirdPerson/Blueprints/BP_ThirdPersonCharacter.PlayerIsInteracting` _asbp_third_person_character))
    (`self.EnableInput` (`GameplayStatics.GetPlayerController` 0))
    (`SceneComponent.SetVisibility` (`self.Take`) true false)))

(event `Key|E`
  (params (Key :type "Key Structure"))
  (bind _item_name (break `/Game/AI/ST_Item_Data` (`self.MyItemData`)))
  (:`Pressed`
    (bind _asbp_third_person_character (cast `/Game/ThirdPerson/Blueprints/BP_ThirdPersonCharacter` (`GameplayStatics.GetPlayerCharacter` 0)))
    (set `self.FoundItem?` false)
    (bind _inventory (`/Game/ThirdPerson/Blueprints/BP_ThirdPersonCharacter.Inventory` _asbp_third_person_character))
    (for (_array_element _array_index) _inventory
      (bind (_item_name_2 _item_mesh _material _item_type _is_rare _item_price _trust_point _count _restore_amount _required_trust) (break `/Game/AI/ST_Item_Data` _array_element))
      (if (`KismetTextLibrary.EqualEqual_TextText` _item_name _item_name_2)
        (set `self.FoundItem?` true)
        (`KismetArrayLibrary.Array_Set` _inventory _array_index (make `/Game/AI/ST_Item_Data` _item_name_2 _item_mesh _material _item_type _is_rare _item_price _trust_point (+ _count 1) _restore_amount _required_trust) true)
        (`KismetSystemLibrary.PrintString` (`KismetTextLibrary.Conv_TextToString` _item_name) true true (struct :`R` 1.0 :`G` 0.155123 :`B` 0.312432 :`A` 1.0) 3.0)
        (`self.SetActorHiddenInGame` true)
        (`self.SetActorEnableCollision` false)
        (break)))
    (if (`self.FoundItem?`)
      (bind _inventorywidgetref (`/Game/ThirdPerson/Blueprints/BP_ThirdPersonCharacter.InventoryWidgetRef` _asbp_third_person_character))
      (`/Engine/EditorBlueprintResources/StandardMacros.IsValid` _inventorywidgetref
        (:`Is Valid`
          (`/Game/AI/WBP_InventoryMain.UpdateInventoryUI` _inventorywidgetref))
        (:`Is Not Valid`
          _))
      (`KismetSystemLibrary.Delay` 60.0)
      (`self.SetActorHiddenInGame` false)
      (`self.SetActorEnableCollision` true)
      (`self.DecideItem`)
      (else
        (`KismetArrayLibrary.Array_Add` _inventory (`self.MyItemData`))
        (`KismetSystemLibrary.PrintString` (`KismetTextLibrary.Conv_TextToString` _item_name) true true (struct :`R` 1.0 :`G` 0.155123 :`B` 0.312432 :`A` 1.0) 3.0)
        (`self.SetActorHiddenInGame` true)
        (`self.SetActorEnableCollision` false)
        (`/Engine/EditorBlueprintResources/StandardMacros.IsValid` _inventorywidgetref
          (:`Is Valid`
            (`/Game/AI/WBP_InventoryMain.UpdateInventoryUI` _inventorywidgetref))
          (:`Is Not Valid`
            _))
        (`KismetSystemLibrary.Delay` 60.0)
        (`self.SetActorHiddenInGame` false)
        (`self.SetActorEnableCollision` true)
        (`self.DecideItem`)))))

(event `self.ReceiveActorEndOverlap`
  (params (OtherActor :type "Actor Object Reference"))
  (cast `/Game/ThirdPerson/Blueprints/BP_ThirdPersonCharacter` OtherActor)
  (`self.DisableInput` (`GameplayStatics.GetPlayerController` 0))
  (`SceneComponent.SetVisibility` (`self.Take`) false false))

(fn `UserConstructionScript`)